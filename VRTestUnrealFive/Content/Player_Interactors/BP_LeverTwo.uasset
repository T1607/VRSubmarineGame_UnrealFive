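; BP_LeverTwo is a VR lever actor that a motion controller can grab, pull and release.
; While held, Tick projects the controller onto the lever's local YZ plane and uses a look-at angle to set the clamped handle roll.
; That angle becomes a power percentage, and each change in its rounded tenth step calls the LeverIsDown and LeverChangedDepth events and plays a haptic pulse on a hand chosen by MotionSource.
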(event `self.ReceiveBeginPlay`
  (`self.CalcCurrentHandlePecent` null))

(event `self.ReceiveTick`
  (params (DeltaSeconds :type "Float (single-precision)"))
  (bind _motioncontroller (`self.motionController`)
    (:`then`
      (bind (_returnvalue_roll _returnvalue_pitch _returnvalue_yaw) (`KismetMathLibrary.BreakRotator` (`KismetMathLibrary.FindLookAtRotation` (* (`KismetMathLibrary.InverseTransformLocation` (`self.GetTransform`) (`SceneComponent.K2_GetComponentLocation` _motioncontroller)) (0.0 1.0 1.0)) (* (`SceneComponent.RelativeLocation` (`self.SM_Lever_Handle`)) (0.0 1.0 1.0)))))
      (bind _returnvalue (`KismetMathLibrary.FClamp` (+ (`KismetMathLibrary.SelectFloat` (- -180.0 _returnvalue_pitch) _returnvalue_pitch (> _returnvalue_yaw 0.0)) 90.0) -130.0 -30.0))
      (set `self.currentValue` _returnvalue)
      (`SceneComponent.K2_SetRelativeRotation` (`self.SM_Lever_Handle`) (`KismetMathLibrary.MakeRotator` _returnvalue) false false)
      (`self.CalcCurrentHandlePecent` _motioncontroller))
    (:`else`)))

(event `/Game/Player_Interactors/BPI_Player_Interaction.Release`
  (params (motionController :type "MotionControllerComponent Object Reference"))
  (if (== motionController (`self.motionController`))
    (bind _output_get (set `self.motionController` null))
    (`KismetSystemLibrary.PrintString` (`KismetSystemLibrary.GetDisplayName` _output_get))))

(event `/Game/Player_Interactors/BPI_Player_Interaction.Grab`
  (params (motionController :type "MotionControllerComponent Object Reference"))
  (bind _output_get (set `self.motionController` motionController))
  (`KismetSystemLibrary.PrintString` (`KismetSystemLibrary.GetDisplayName` _output_get)))

(fn `CalcCurrentHandlePecent`
  (params (motionController :type "MotionControllerComponent Object Reference"))
  (bind _minvalue (`self.minValue`))
  (bind _returnvalue (/ (+ (`self.currentValue`) (`KismetMathLibrary.Abs` _minvalue)) (`KismetMathLibrary.Abs` (- _minvalue (`self.topValue`)))))
  (bind _returnvalue_2 (`KismetMathLibrary.Round` (* _returnvalue 10.0)))
  (set `self.powerPrecentage` _returnvalue)
  (if (!= _returnvalue_2 (`self.lastDepthTick`))
    (set `self.lastDepthTick` _returnvalue_2)
    (`self.LeverIsDown`)
    (`KismetSystemLibrary.PrintString` (`KismetStringLibrary.Conv_IntToString` (`self.lastDepthTick`)))
    (if (== (`MotionControllerComponent.MotionSource` motionController) "Right")
      (set `self.handInteracting` "Right")
      (else
        (set `self.handInteracting` "Left")))
    (`PlayerController.PlayHapticEffect` (`GameplayStatics.GetPlayerController` 0) "/Game/VRTemplate/Haptics/PistolFireHapticEffect.PistolFireHapticEffect" (`self.handInteracting`) 1.0 false)
    (`self.LeverChangedDepth`)))

(fn `UserConstructionScript`)