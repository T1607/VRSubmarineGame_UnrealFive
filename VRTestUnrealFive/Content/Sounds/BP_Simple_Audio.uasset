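; Central audio actor for a submarine game, playing ambience, horror, engine, Narina, death and win sounds through separate audio components.
; BeginPlay starts the ambience and engine loops, then binds to events on BP_Sub_Route and BP_LeverTwo.
; Speed changes scale engine volume by normalized absolute speed and restart stopped secondary ambience, while the depth lever triggers Narina audio.
; DeathRush plays the death sound and stops ambience, engine and Narina; WinAnnouncement plays the win sound.
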(event `self.ReceiveBeginPlay`
  (bind _ambienceaudio (`self.AmbienceAudio`))
  (bind _ambiencetwoaudio (`self.AmbienceTwoAudio`))
  (bind _ambiencehorroraudio (`self.AmbienceHorrorAudio`))
  (bind _engineaudio (`self.EngineAudio`))
  (`|ExecutionSequence`
    (:`then_0`
      (`AudioComponent.SetSound` _ambienceaudio (`self.ambienceOne`))
      (`AudioComponent.Play` _ambienceaudio 0.0)
      (`AudioComponent.SetSound` _ambiencetwoaudio (`self.ambienceTwo`))
      (`AudioComponent.Play` _ambiencetwoaudio 0.0)
      (`AudioComponent.SetSound` _ambiencehorroraudio (`self.ambienceHorror`))
      (`AudioComponent.Play` _ambiencehorroraudio 0.0)
      (`AudioComponent.SetSound` _engineaudio (`self.engine`))
      (`AudioComponent.Play` _engineaudio 0.0))
    (:`then_1`
      (bind _returnvalue (`GameplayStatics.GetActorOfClass` "/Game/Submarine_Logic/BP_Sub_Route.BP_Sub_Route_C"))
      (set `self.subRoute` _returnvalue)
      (add `/Game/Submarine_Logic/BP_Sub_Route.changeInMoveSpeed` (`self.subRoute`) (delegate `ChangeEngineVolume`)))
    (:`then_2`
      (bind _returnvalue_2 (`GameplayStatics.GetActorOfClass` "/Game/Player_Interactors/BP_LeverTwo.BP_LeverTwo_C"))
      (set `self.depthLever` _returnvalue_2)
      (add `/Game/Player_Interactors/BP_LeverTwo.LeverIsDown` (`self.depthLever`) (delegate `PlayNarinaAudio`)))))

(event `ChangeEngineVolume`
  (bind _ambiencetwoaudio (`self.AmbienceTwoAudio`))
  (`self.engineVolumeChange`)
  (if (not (`AudioComponent.IsPlaying` _ambiencetwoaudio))
    (`AudioComponent.SetSound` _ambiencetwoaudio (`self.ambienceTwo`))
    (`AudioComponent.Play` _ambiencetwoaudio 0.0)))

(event `self.ReceiveTick`
  (params (DeltaSeconds :type "Float (single-precision)")))

(event `PlayNarinaAudio`
  (bind _narinaaudio (`self.NarinaAudio`))
  (if (not (`AudioComponent.IsPlaying` _narinaaudio))
    (`AudioComponent.SetSound` _narinaaudio (`self.narina`))
    (`AudioComponent.Play` _narinaaudio 0.0)))

(event `DeathRush`
  (bind _deathaudio (`self.DeathAudio`))
  (`AudioComponent.SetSound` _deathaudio (`self.death`))
  (`AudioComponent.Play` _deathaudio 0.0)
  (`AudioComponent.Stop` (`self.AmbienceAudio`))
  (`AudioComponent.Stop` (`self.AmbienceTwoAudio`))
  (`AudioComponent.Stop` (`self.NarinaAudio`))
  (`AudioComponent.Stop` (`self.EngineAudio`))
  (`AudioComponent.Stop` (`self.AmbienceHorrorAudio`)))

(event `WinAnnouncement`
  (bind _winaudio (`self.WinAudio`))
  (`AudioComponent.SetSound` _winaudio (`self.win`))
  (`AudioComponent.Play` _winaudio 0.0))

(fn `engineVolumeChange`
  (bind _subroute (`self.subRoute`))
  (set `self.engineVolume` (/ (`KismetMathLibrary.Abs` (`/Game/Submarine_Logic/BP_Sub_Route.currentMoveSpeed` _subroute)) (`/Game/Submarine_Logic/BP_Sub_Route.maxMoveSpeed` _subroute)))
  (`AudioComponent.SetVolumeMultiplier` (`self.EngineAudio`) (`self.engineVolume`)))

(fn `UserConstructionScript`)