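; BP_Sub_Depth simulates the submarine's depth control against a scrolling environment, calling a death sequence when the sub hits tagged environment geometry.
; Emerge and submerge events step a vertical speed up or down within a symmetric limit, applied as physics linear velocity along the sub's up vector.
; Forward travel is faked: Tick sweeps the environment along Y by a per-frame scroll speed, updated whenever BP_Sub_Route signals a speed change.
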(event `self.ReceiveBeginPlay`
  (bind _returnvalue (`GameplayStatics.GetActorOfClass` "/Game/Submarine_Logic/BP_Sub_Route.BP_Sub_Route_C"))
  (bind _output_get (set `self.subRoute` _returnvalue))
  (add `/Game/Submarine_Logic/BP_Sub_Route.changeInMoveSpeed` _output_get (delegate `UpdateScrollSpeed`)))

(event `UpdateScrollSpeed`
  (set `self.scrollSpeed` (`/Game/Submarine_Logic/BP_Sub_Route.currentMoveSpeed` (`self.subRoute`))))

(event `/Game/Submarine_Logic/BPI_Interaction.emergeSubmarine`
  (bind _maxdepthchange (`self.maxDepthChange`))
  (bind _returnvalue (+ (`self.currentDepthChange`) (`self.depthChangeSpeed`)))
  (if (>= _returnvalue _maxdepthchange)
    (set `self.currentDepthChange` _maxdepthchange)
    (else
      (set `self.currentDepthChange` _returnvalue)))
  (`self.depthChange` :!label _label))

(event `/Game/Submarine_Logic/BPI_Interaction.submergeSubmarine`
  (bind _returnvalue (* (`self.maxDepthChange`) -1.0))
  (bind _returnvalue_2 (+ (`self.currentDepthChange`) (* (`self.depthChangeSpeed`) -1.0)))
  (if (>= _returnvalue _returnvalue_2)
    (set `self.currentDepthChange` _returnvalue)
    (goto _label)
    (else
      (set `self.currentDepthChange` _returnvalue_2)
      (goto _label))))

(event `self.SubParent.OnComponentHit`
  (params (HitComponent :type "PrimitiveComponent Object Reference") (OtherActor :type "Actor Object Reference") (OtherComp :type "PrimitiveComponent Object Reference") (NormalImpulse :type "Vector Structure") (Hit :type "HitResult Structure (by ref)"))
  (if (`ActorComponent.ComponentHasTag` OtherComp "Enviornment")
    (`self.deathSequence`)))

(event `self.ReceiveTick`
  (params (DeltaSeconds :type "Float (single-precision)"))
  (bind _enviornment (`self.Enviornment`))
  (bind _scrollspeed (`self.scrollSpeed`))
  (bind (_relativelocation_x _relativelocation_y _relativelocation_z) (`KismetMathLibrary.BreakVector` (`SceneComponent.RelativeLocation` _enviornment)))
  (if (!= _scrollspeed 0.0)
    (`SceneComponent.K2_SetRelativeLocation` _enviornment (`KismetMathLibrary.MakeVector` _relativelocation_x (+ _relativelocation_y _scrollspeed) _relativelocation_z) true false)))

(fn `depthChange`
  (bind _subparent (`self.SubParent`))
  (`PrimitiveComponent.SetPhysicsLinearVelocity` _subparent (* (`self.currentDepthChange`) (`SceneComponent.GetUpVector` _subparent)) false "None"))

(fn `UserConstructionScript`)