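; BP_Sub_Route is a steerable submarine that dies on hitting "Enviornment"-tagged components and wins on hitting "Win"-tagged ones.
; Turn events adjust SubParent's relative roll, while forward and backward events step CurrentMoveSpeed within plus or minus MaxMoveSpeed.
; Each input then sets physics velocity along SubParent's up vector and calls CallChangeInMoveSpeed, so movement updates on events rather than Tick.
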(event `self.ReceiveBeginPlay`)

(event `self.ReceiveTick`
  (params (DeltaSeconds :type "Float (single-precision)")))

(event `/Game/Submarine_Logic/BPI_Interaction.TurnSubmarineRight`
  (`self.turnSubRight` (`self.turnRate`)))

(event `/Game/Submarine_Logic/BPI_Interaction.TurnSubmarineLeft`
  (`self.turnSubLeft` (`self.turnRate`)))

(event `/Game/Submarine_Logic/BPI_Interaction.moveSubmarineForward`
  (`self.calcMoveForward`))

(event `/Game/Submarine_Logic/BPI_Interaction.moveSubmarineBackward`
  (`self.calcMoveBack`))

(event `self.SubParent.OnComponentHit`
  (params (HitComponent :type "PrimitiveComponent Object Reference") (OtherActor :type "Actor Object Reference") (OtherComp :type "PrimitiveComponent Object Reference") (NormalImpulse :type "Vector Structure") (Hit :type "HitResult Structure (by ref)"))
  (if (`ActorComponent.ComponentHasTag` OtherComp "Enviornment")
    (`self.deathSequence`)
    (elif (`ActorComponent.ComponentHasTag` OtherComp "Win")
      (`self.winSequence`))))

(fn `calcMoveBack`
  (bind _returnvalue (* (`self.maxMoveSpeed`) -1.0))
  (bind _returnvalue_2 (+ (`self.currentMoveSpeed`) (* (`self.moveChangeSpeed`) -1.0)))
  (if (>= _returnvalue _returnvalue_2)
    (set `self.currentMoveSpeed` _returnvalue)
    (else
      (set `self.currentMoveSpeed` _returnvalue_2)))
  (`self.moveSubmarine`))

(fn `calcMoveForward`
  (bind _maxmovespeed (`self.maxMoveSpeed`))
  (bind _returnvalue (+ (`self.currentMoveSpeed`) (`self.moveChangeSpeed`)))
  (if (>= _returnvalue _maxmovespeed)
    (set `self.currentMoveSpeed` _maxmovespeed)
    (else
      (set `self.currentMoveSpeed` _returnvalue)))
  (`self.moveSubmarine`))

(fn `moveSubmarine`
  (bind _subparent (`self.SubParent`))
  (`PrimitiveComponent.SetPhysicsLinearVelocity` _subparent (* (`self.currentMoveSpeed`) (`SceneComponent.GetUpVector` _subparent)) false "None")
  (`self.changeInMoveSpeed`))

(fn `turnSubLeft`
  (params (`turn input` :type "Float (double-precision)"))
  (bind _subparent (`self.SubParent`))
  (bind (_relativerotation_roll _relativerotation_pitch _relativerotation_yaw) (`KismetMathLibrary.BreakRotator` (`SceneComponent.RelativeRotation` _subparent)))
  (`SceneComponent.K2_SetRelativeRotation` _subparent (`KismetMathLibrary.MakeRotator` (+ (* `turn input` -1.0) _relativerotation_roll) _relativerotation_pitch _relativerotation_yaw) false false)
  (`self.moveSubmarine`))

(fn `turnSubRight`
  (params (`turn input` :type "Float (double-precision)"))
  (bind _subparent (`self.SubParent`))
  (bind (_relativerotation_roll _relativerotation_pitch _relativerotation_yaw) (`KismetMathLibrary.BreakRotator` (`SceneComponent.RelativeRotation` _subparent)))
  (`SceneComponent.K2_SetRelativeRotation` _subparent (`KismetMathLibrary.MakeRotator` (+ `turn input` _relativerotation_roll) _relativerotation_pitch _relativerotation_yaw) false false)
  (`self.moveSubmarine`))

(fn `UserConstructionScript`)